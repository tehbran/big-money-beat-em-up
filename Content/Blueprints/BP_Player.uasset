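; Player character that walks, punches other players and drops its money on death.
; Punch input toggles a hand-socketed collision that damages overlapped BP_Player capsules, scaling with carried Money.
; At zero health it ragdolls, spawns BP_Money holding its Money, then destroys itself after a delay.
; Tick sets yaw from a mouse-ray plane intersection, but only while health is zero or below.
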(event OnComponentBeginOverlap(RightHandCollision)
  (params (OverlappedComponent :type Primitive%20Component%20Object%20Reference) (OtherActor :type Actor%20Object%20Reference) (OtherComp :type Primitive%20Component%20Object%20Reference) (OtherBodyIndex :type Integer) (bFromSweep :type Boolean) (SweepResult :type Hit%20Result%20Structure%20%28by%20ref%29))
  (bind _asbp_player (Utilities|Casting|CastToBP_Player OtherActor))
  (if (Math|Boolean|ANDBoolean (Variables|Default|GetIsPunching) (== OtherComp (Variables|/Script/Engine.Character|GetCapsuleComponent _asbp_player)) (not (== (Variables|/Script/Engine.Character|GetCapsuleComponent _asbp_player) (Variables|Collision|GetCapsuleComponent self))))
    (Game|Damage|ApplyDamage _asbp_player (+ 1e+01 (* 0.6 (Variables|Default|GetMoney))) (Pawn|GetController (Variables|Actor|GetInstigator)) 0)
    (Development|PrintString "Gave Damage")
    (Utilities|FlowControl|Delay 1.0)))

(event EventBeginPlay)

(event Collision|EventActorBeginOverlap
  (params (OtherActor :type Actor%20Object%20Reference)))

(event EventTick
  (params (DeltaSeconds :type Float%20%28single-precision%29))
  (bind _returnvalue (Game|GetPlayerController 0))
  (bind (_worldlocation _worlddirection) (Game|Player|ConvertMouseLocationToWorldSpace _returnvalue))
  (if (<= (Variables|Default|GetCurrentHealth) 0.0)
    (Transformation|SetActorRotation (Math|Rotator|MakeRotator 0.0 0.0 (.yaw (Math|Rotator|FindLookatRotation (Math|Vector|MakeVector 0.0 0.0 0.0) (.Intersection (Class|KismetMathLibrary|LinePlaneIntersectionOriginNormal _worldlocation (+ (* _worlddirection 5e+03) _worldlocation) (Transformation|GetActorLocation) "0, 0, 0"))))))))

(event Game|Damage|EventAnyDamage
  (params (Damage :type Float%20%28single-precision%29) (DamageType :type Damage%20Type%20Object%20Reference) (InstigatedBy :type Controller%20Object%20Reference) (DamageCauser :type Actor%20Object%20Reference))
  (bind _mesh (Variables|Character|GetMesh))
  (bind _output_get (Variables|Default|SetCurrentHealth (Math|Float|Clamp(Float) (- (Variables|Default|GetCurrentHealth) Damage) 0.0 (Variables|Default|GetMaxHealth))))
  (Development|PrintString (Utilities|String|Append "Health: " (Utilities|String|ToString(Float) _output_get)))
  (if (<= (Variables|Default|GetCurrentHealth) 0.0)
    (Collision|SetCollisionResponsetoChannel (Variables|Collision|GetCapsuleComponent) "ECC_GameTraceChannel2" "ECR_Ignore")
    (Collision|SetCollisionProfileName _mesh "DeadChar" :!class /Script/Engine.PrimitiveComponent)
    (Physics|SetSimulatePhysics _mesh true)
    (CallFunction|SpawnMoney)
    (Utilities|FlowControl|Delay 5.0)
    (Actor|DestroyActor)))

(event Collision|EventHit
  (params (MyComp :type Primitive%20Component%20Object%20Reference) (Other :type Actor%20Object%20Reference) (OtherComp :type Primitive%20Component%20Object%20Reference) (bSelfMoved :type Boolean) (HitLocation :type Vector :default "0, 0, 0") (HitNormal :type Vector :default "0, 0, 0") (NormalImpulse :type Vector :default "0, 0, 0") (Hit :type Hit%20Result%20Structure%20%28by%20ref%29)))

(event Input|ActionEvents|InputActionPunch
  (params (Key :type Key%20Structure :default "None"))
  (bind _righthandcollision (Variables|Default|GetRightHandCollision))
  (:Pressed
    (Variables|Default|SetIsPunching true)
    (Collision|SetCollisionEnabled _righthandcollision "QueryAndPhysics"))
  (:Released
    (Variables|Default|SetIsPunching false)
    (Collision|SetCollisionEnabled _righthandcollision "NoCollision")
    (Utilities|FlowControl|Delay 1.25)))

(event Input|AxisEvents|InputAxisWalkForward
  (params (AxisValue :type Float%20%28single-precision%29))
  (Pawn|Input|AddMovementInput (Math|Vector|GetForwardVector (Pawn|GetControlRotation :!class /Script/Engine.Pawn)) AxisValue false))

(event Input|AxisEvents|InputAxisWalkRight
  (params (AxisValue :type Float%20%28single-precision%29))
  (Pawn|Input|AddMovementInput (Math|Vector|GetRightVector (Pawn|GetControlRotation :!class /Script/Engine.Pawn)) AxisValue false))

(fn ConstructionScript
  (Transformation|AttachComponentToComponent (Variables|Default|GetRightHandCollision) (Variables|Character|GetMesh) "hand_r" "SnapToTarget" "KeepRelative" "KeepRelative" true))

(fn SpawnMoney
  (bind _returnvalue (Game|SpawnActorfromClass "/Game/Blueprints/BP_Money.BP_Money_C" (Math|Conversions|ToTransform(Vector) (Math|Transform|TransformLocation (Math|Transform|MakeTransform "0, 0,100.000000") (Transformation|GetActorLocation))) "Undefined" 0 0))
  (bind _output_get (Variables|Default|SetMoneySpawn _returnvalue))
  (Variables|/Game/Blueprints/BP_Money.BP_Money_C|SetMoneyValue _output_get (Variables|Default|GetMoney)))