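; BP_Money is a cash pickup actor that the player collects by overlapping its WadOfCash component.
; It casts both the overlapping actor and player pawn 0 to BP_Player and proceeds only if they match.
; MoneyValue is added to the player's Money, MaxHealth and CurrentHealth alike, so cash also grows health.
; It then prints the new money total, labeled as "Gained", and destroys itself.
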(event OnComponentBeginOverlap(WadOfCash)
  (params (OverlappedComponent :type Primitive%20Component%20Object%20Reference) (OtherActor :type Actor%20Object%20Reference) (OtherComp :type Primitive%20Component%20Object%20Reference) (OtherBodyIndex :type Integer) (bFromSweep :type Boolean) (SweepResult :type Hit%20Result%20Structure%20%28by%20ref%29))
  (bind _moneyvalue (Variables|Default|GetMoneyValue))
  (bind _asbp_player (Utilities|Casting|CastToBP_Player OtherActor))
  (bind _asbp_player_2 (Utilities|Casting|CastToBP_Player (Game|Player|GetPlayerPawn 0)))
  (if (== _asbp_player_2 _asbp_player)
    (bind _output_get (Variables|/Game/Blueprints/BP_Player.BP_Player_C|SetMoney _asbp_player_2 (+ (Variables|/Game/Blueprints/BP_Player.BP_Player_C|GetMoney _asbp_player_2) _moneyvalue)))
    (Variables|/Game/Blueprints/BP_Player.BP_Player_C|SetMaxHealth _asbp_player_2 (+ (Variables|/Game/Blueprints/BP_Player.BP_Player_C|GetMaxHealth _asbp_player_2) _moneyvalue))
    (Variables|/Game/Blueprints/BP_Player.BP_Player_C|SetCurrentHealth _asbp_player_2 (+ _moneyvalue (Variables|/Game/Blueprints/BP_Player.BP_Player_C|GetCurrentHealth _asbp_player_2)))
    (Development|PrintString (Utilities|String|Append "Gained $" (Utilities|String|ToString(Float) _output_get)))
    (Actor|DestroyActor)))

(event EventBeginPlay)

(event Collision|EventActorBeginOverlap
  (params (OtherActor :type Actor%20Object%20Reference)))

(event EventTick
  (params (DeltaSeconds :type Float%20%28single-precision%29)))

(fn ConstructionScript)