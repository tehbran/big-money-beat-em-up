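; BP_WorldLooper builds a looping world by chaining BP_WorldLoop city sections one after another.
; On BeginPlay it spawns three sections, the first offset from the player pawn and set as oldest, with its NextAreaTrigger set to block all channels.
; Each further section spawns at the newest one's SpawnPoint, updating the current and newest references.
; Every section receives a Looper reference back to this actor.
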(event EventBeginPlay
  (CallFunction|SpawnInitialSections))

(event Collision|EventActorBeginOverlap
  (params (OtherActor :type Actor%20Object%20Reference)))

(event EventTick
  (params (DeltaSeconds :type Float%20%28single-precision%29)))

(fn ConstructionScript)

(fn SpawnCitySection
  (params (SpawnNextLocation :type Vector))
  (bind _returnvalue (Game|SpawnActorfromClass "/Game/Blueprints/BP_WorldLoop.BP_WorldLoop_C" (Math|Transform|MakeTransform SpawnNextLocation "0, 0, 0" "1,1,1") "Undefined" 0 0))
  (bind _output_get (Variables|Default|SetNewestSection _returnvalue))
  (Variables|/Game/Blueprints/BP_WorldLoop.BP_WorldLoop_C|SetLooper _output_get self))

(fn SpawnSectionatTrigger
  (bind _newestsection (Variables|Default|GetNewestSection))
  (if (== (Variables|Default|GetOldestSection) _newestsection)
    _
    (else
      (Variables|Default|SetCurrent%20Section _newestsection)))
  (CallFunction|SpawnCitySection (Transformation|GetWorldLocation (Variables|/Game/Blueprints/BP_WorldLoop.BP_WorldLoop_C|GetSpawnPoint _newestsection))))

(fn SpawnInitialSections
  (for _index (range 0 2)
    (Utilities|IsValid (Variables|Default|GetNewestSection)
      (:Is%20Valid
        (CallFunction|SpawnSectionatTrigger))
      (:Is%20Not%20Valid
        (CallFunction|SpawnCitySection (Math|Transform|TransformLocation (Math|Transform|MakeTransform "-2200.000000, 0,-10.000000") (Transformation|GetActorLocation (Game|Player|GetPlayerPawn 0))))
        (bind _output_get (Variables|Default|SetOldestSection (Variables|Default|GetNewestSection)))
        (Collision|SetCollisionResponsetoAllChannels (Variables|/Game/Blueprints/BP_WorldLoop.BP_WorldLoop_C|GetNextAreaTrigger _output_get) "ECR_Block")))))